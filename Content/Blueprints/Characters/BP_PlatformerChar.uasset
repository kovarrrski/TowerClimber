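; Platformer 2D sprite character Blueprint that handles the character's defeat.
; Defeat runs once, guarded by IsDefeated, disabling capsule collision and the movement plane constraint so the character can leave the 2D plane.
; LaunchOnDefeat throws it up and along world right using tunable strengths.
; The anim instance jumps to the defeated node, and a raised translucent sort priority adjusts sprite draw order as it flies toward the camera.
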(event `Defeat`
  ;[1 1 1] The function eveluate Is Deafeated char? (if not not defeated - then defeated)
  (if (not (`self.IsDefeated`))
    (set `self.IsDefeated` true)
    ;[1 1 1] Char lose collision
    (`PrimitiveComponent.SetCollisionEnabled` (`self.CapsuleComponent`) "NoCollision")
    ;[1 1 1] Char is not moving in the air???
    (`MovementComponent.SetPlaneConstraintEnabled` (`self.CharacterMovement`) false)
    (`self.LaunchOnDefeat`)
    ;[1 1 1] Play defeted anim from Locomotion
    (`PaperZDAnimInstance.JumpToNode` (`self.GetAnimInstance`) "JumpDefeated" "None")
    ;[1 1 1] Translucency of the defeated Char that flighs in forward to Camera
    (`PrimitiveComponent.SetTranslucentSortPriority` (`self.Sprite`) 10)))

(fn `LaunchOnDefeat`
  ;[1 1 1] Video 69. 6min. Bounce and fligh up away when touch Pig
  (`self.LaunchCharacter` (+ (* (`KismetMathLibrary.Vector_Up`) (`self.DefeatUpLaunch`)) (* (`KismetMathLibrary.Vector_Right`) (`self.DefeatForwardLaunch`))) true true))

(fn `UserConstructionScript`)