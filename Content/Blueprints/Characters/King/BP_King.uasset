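; BP_King is the player-controlled 2D platformer hero, moving along X and turning to face its direction.
; Jumping adds input buffering and coyote time through retriggerable delays and a CanJumpInternal override.
; While airborne, downward traces switch the capsule's platform-channel response, blocking only when descending onto a platform.
; Falling onto a BP_Pig defeats it and bounces the King; other pig contact defeats the King, removing input, detaching the camera and playing shake and sound.
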(event `self.ReceiveBeginPlay`
  (`parent.ReceiveBeginPlay`)
  (bind _asplayer_controller (cast `PlayerController` (`self.GetController`)))
  (`EnhancedInputSubsystemInterface.AddMappingContext` (pcsubsystem `EnhancedInputLocalPlayerSubsystem` _asplayer_controller) "/Game/Input/IMC_Platformer.IMC_Platformer" 0 (struct)))

(event `self.ReceiveTick`
  (params (DeltaSeconds :type "Float (single-precision)"))
  ;[1 1 1] Called check Rotation of Char with L/R movement every Frame
  (`parent.ReceiveTick` DeltaSeconds)
  (`self.UpdateControllerRotation`)
  (`self.TraceForPlatforms`)
  ;[1 1 1] for jump buffering?
  (if (and (`self.IsJumpBuffering`) (`self.CanJump`))
    (`self.Jump`)))

(event `EnhancedInput|/Game/Input/Actions/IA_Jump`
  (params (ActionValue :type Boolean) (ElapsedSeconds :type "Float (double-precision)") (TriggeredSeconds :type "Float (double-precision)") (InputAction :type "InputAction Object Reference" :default "/Game/Input/Actions/IA_Jump.IA_Jump"))
  (:`Started`
    (if (`self.CanJump`)
      (`self.Jump`)
      (else
        ;[1 1 1] Jump Buffering in the air
        (set `self.IsJumpBuffering` true)
        (`KismetSystemLibrary.RetriggerableDelay` (`self.JumpBufferLenght`))
        (set `self.IsJumpBuffering` false))))
  (:`Completed`
    (`self.StopJumping`)))

(event `EnhancedInput|/Game/Input/Actions/IA_Move`
  (params (ActionValue :type "Float (double-precision)") (ElapsedSeconds :type "Float (double-precision)") (TriggeredSeconds :type "Float (double-precision)") (InputAction :type "InputAction Object Reference" :default "/Game/Input/Actions/IA_Move.IA_Move"))
  (:`Triggered`
    (`self.AddMovementInput` (1.0 0.0 0.0) ActionValue)))

(event `self.CapsuleComponent.OnComponentBeginOverlap`
  (params (OverlappedComponent :type "PrimitiveComponent Object Reference") (OtherActor :type "Actor Object Reference") (OtherComp :type "PrimitiveComponent Object Reference") (OtherBodyIndex :type Integer) (bFromSweep :type Boolean) (SweepResult :type "HitResult Structure (by ref)"))
  (bind (_returnvalue_x _returnvalue_y _returnvalue_z) (`KismetMathLibrary.BreakVector` (`self.GetVelocity`)))
  ;[1 1 1] If King touched the Pig (Overlapped Capsules) then King become Defeated
  (bind _asbp_pig (cast `/Game/Blueprints/Characters/Pig/BP_Pig` OtherActor))
  ;[1 1 1] if Jump on top of the Pig - pig Defeated
  (if (and (`NavMovementComponent.IsFalling` (`self.CharacterMovement`)) (< _returnvalue_z 0.0))
    (`self.Defeat` _asbp_pig)
    ;[1 1 1] For Bouncing up when kill the Pig
    (`self.LaunchCharacter` (`KismetMathLibrary.MakeVector` 0.0 0.0 (`self.EnemyBounceLaunch`)) false true)
    (else
      (`self.Defeat`))))

(event `self.Defeat`
  ;[1 1 1] Call function from Parent BP (flight up and forward when Overlap Pig box)
  (`parent.Defeat`)
  ;[1 1 1] Make Input invalid after Death of King (Overlapping of Pig Box Collision)
  (bind _asplayer_controller (cast `PlayerController` (`self.GetController`)))
  (`EnhancedInputSubsystemInterface.RemoveMappingContext` (pcsubsystem `EnhancedInputLocalPlayerSubsystem` _asplayer_controller) "/Game/Input/IMC_Platformer.IMC_Platformer" (struct))
  ;[1 1 1] Off the Camera's Following by the King after his Death
  (`SceneComponent.K2_DetachFromComponent` (`self.SpringArm`) "KeepWorld" "KeepRelative" "KeepRelative" true)
  ;[1 1 1] Defeated Sound
  (`GameplayStatics.PlaySound2D` "/Game/Sounds/PlayerDefeated/S_PlayerDefeated_Cue.S_PlayerDefeated_Cue" 1.0 1.0 0.0 null null)
  ;[1 1 1] Camera Shaking around death Scene
  (`GameplayStatics.PlayWorldCameraShake` "/Game/CameraShake/CS_Defeated.CS_Defeated_C" (`self.K2_GetActorLocation`) 0.0 10000.0))

(event `self.OnWalkingOffLedge`
  (params (PreviousFloorImpactNormal :type "Vector Structure (by ref)") (PreviousFloorContactNormal :type "Vector Structure (by ref)") (PreviousLocation :type "Vector Structure (by ref)") (TimeDelta :type "Float (single-precision)"))
  ;[1 1 1] Coyote Time delay Setting/ King walks out of the ledge, King in CoyoteTime, when 0.2sec passed, King is not in CoyoteTime anymore
  (set `self.IsInCoyoteTime` true)
  (`KismetSystemLibrary.RetriggerableDelay` (`self.CoyoteTimeLenght`))
  (set `self.IsInCoyoteTime` false))

(fn `CanJumpInternal`
  (returns (ReturnValue :type Boolean))
  ;[1 1 1] Something about jumping from the Edge
  (bind _returnvalue (`parent.CanJumpInternal`))
  (return (or _returnvalue (`self.IsInCoyoteTime`))))

(fn `TraceForPlatforms`
  (bind (_returnvalue_x _returnvalue_y _returnvalue_z) (`KismetMathLibrary.BreakVector` (`self.GetVelocity`)))
  (bind _returnvalue (`SceneComponent.K2_GetComponentLocation` (`self.FootPosition`)))
  ;[1 1 1] Проверяет трейсом платформы, но почему под ногами, ничего не понимаю. Detection of the object below the King
  (if (`NavMovementComponent.IsFalling` (`self.CharacterMovement`))
    (bind (_outhits _returnvalue_2) (`KismetSystemLibrary.LineTraceMultiForObjects` _returnvalue (+ _returnvalue (* (`KismetMathLibrary.Vector_Down`) (`self.PlatformCheckDistance`))) (`|MakeArray` "ObjectTypeQuery7" :!type "EObjectTypeQuery Enum")))
    (if (and _returnvalue_2 (< _returnvalue_z 0.0))
      ;[1 1 1] If King has a platform below - the platform become a block (in jump tracing mode)
      (`PrimitiveComponent.SetCollisionResponseToChannel` (`self.CapsuleComponent`) "ECC_GameTraceChannel1" "ECR_Block")
      (else
        ;[1 1 1] If King has no platform below - he go through Object (in jump tracing mode)?????
        (`PrimitiveComponent.SetCollisionResponseToChannel` (`self.CapsuleComponent`) "ECC_GameTraceChannel1" "ECR_Overlap")))))

(fn `UpdateControllerRotation`
  (bind _returnvalue (`self.GetController`))
  (bind _returnvalue_2 (`self.GetController`))
  (bind _velocity_x (`KismetMathLibrary.BreakVector` (`MovementComponent.Velocity` (`self.CharacterMovement`))))
  ;[1 1 1] Rotation of Char depends of L/R movements
  (`/Engine/EditorBlueprintResources/StandardMacros.CompareFloat` _velocity_x
    (:`>`
      (`/Engine/EditorBlueprintResources/StandardMacros.IsValid` _returnvalue_2
        (:`Is Valid`
          (`Controller.SetControlRotation` _returnvalue_2 (`KismetMathLibrary.MakeRotator` 0.0)))))
    (:`<`
      ;;[1 1 1] Rotation of Pawn (on Z axis) in Left Direction if X<0
      (`/Engine/EditorBlueprintResources/StandardMacros.IsValid` _returnvalue
        (:`Is Valid`
          (`Controller.SetControlRotation` _returnvalue (`KismetMathLibrary.MakeRotator` 0.0 0.0 180.0)))))))

(fn `UserConstructionScript`
  (`parent.UserConstructionScript`))